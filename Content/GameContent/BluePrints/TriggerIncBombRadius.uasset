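; Bomb radius power-up trigger for a Bomberman game that raises the player's bomb radius when picked up.
; BeginPlay caches the first player's bomberman, its player controller (otherwise unused here) and the bmGameState.
; Any actor overlap, with no check on the overlapping actor, increments that cached bomberman's radius, calls BmDestroyPowerUp on the game state, then destroys the trigger.
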(event EventBeginPlay
  (bind _asbomberman (Utilities|Casting|CastTobomberman (Game|GetPlayerCharacter 0)))
  (Variables|Default|SetbombermanRef _asbomberman)
  (bind _asbomberman_player_controller (Utilities|Casting|CastToBombermanPlayerController (Game|GetPlayerController 0)))
  (Variables|Default|SetbmPlayerControllerRef _asbomberman_player_controller)
  (bind _asbm_game_state (Utilities|Casting|CastTobmGameState (Game|GetGameState)))
  (Variables|Default|SetbmGameStateRef _asbm_game_state))

(event Collision|EventActorBeginOverlap
  (params (OtherActor :type Actor%20Object%20Reference))
  (Development|PrintString "powered UP from trigger")
  (Math|Integer|IncrementInt (Variables|/Game/GameContent/BluePrints/bomberman.bomberman_C|GetbmBombRadius (Variables|Default|GetbombermanRef))
    (:%20%20
      (Default|BmDestroyPowerUp (Variables|Default|GetbmGameStateRef) self)
      (Actor|DestroyActor))))

(event EventTick
  (params (DeltaSeconds :type Float%20%28single-precision%29)))

(fn ConstructionScript)