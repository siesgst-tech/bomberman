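; Bomberman player character that handles world-axis movement, bomb placement, lives and death, with an unfinished bomb-kick input.
; Bombs snap to the grid cell the player faces, rejecting diagonal facings and cells holding crates or fixed boxes.
; Placement goes directly to the game state on authority or through the player controller on remote, decrementing the bomb count.
; Damage updates health through the controller; death detaches and hides the character.
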(event Custom|Increase%20Bombs
  ;[0.3134 1 0] Increase Bombs
  (Variables|Default|SetbmBombPresent (+ (Variables|Default|GetbmBombPresent) 1)))

(event Custom|Take%20Damage
  ;[1 1 1] Take Damage
  (if (> (Variables|Default|GetbmPlayerLife) 1)
    (bind _output_get (Variables|Default|SetbmPlayerLife (- (Variables|Default|GetbmPlayerLife) 1)))
    (Development|PrintString (Utilities|String|Append "Player Life" (Utilities|String|ToString(Integer) _output_get)))
    (else
      (Variables|Default|SetbmPlayerLife (- (Variables|Default|GetbmPlayerLife) 1))
      (Development|PrintString "Player is dead")
      (CallFunction|Die)))
  (bind _asbomberman_player_controller (Utilities|Casting|CastToBombermanPlayerController (Pawn|GetController)))
  (Default|UpdateHealth _asbomberman_player_controller (Variables|Default|GetbmPlayerLife)))

(event Custom|Die
  ;[1 1 1] Player Death Event
  (Class|Pawn|DetachfromControllerPendingDestroy)
  (Development|SetHiddeninGame (Variables|Collision|GetCapsuleComponent) true false))

(event EventBeginPlay
  ;[1 0.217 0.7479] initializing references
  (bind _asbm_game_state (Utilities|Casting|CastTobmGameState (Game|GetGameState)))
  (Variables|Default|SetbmGameStateRef _asbm_game_state)
  (bind _asbm_game_instance (Utilities|Casting|CastTobmGameInstance (Game|GetGameInstance)))
  (Variables|Default|SetgmGameInstRef _asbm_game_instance)
  (Development|PrintString (Utilities|String|Append (Utilities|String|ToString(Integer) (Variables|Default|GetbmBombPresent)) (Utilities|String|ToString(Integer) (Variables|Default|GetbmBombRadius)) (Utilities|String|ToString(Integer) (Variables|Default|GetbmPlayerLife))) true true "(R=1.000000,G=0.758435,B=0.005604,A=1.000000)" 1e+01)
  (bind _asbomberman_player_controller (Utilities|Casting|CastToBombermanPlayerController (Pawn|GetController)))
  (Default|UpdateHealth _asbomberman_player_controller (Variables|Default|GetbmPlayerLife)))

(event Input|ActionEvents|InputActionkickBomb
  (params (Key :type Key%20Structure :default "AnyKey"))
  ;[1 1 1] kicking bomb powerup (need to be worked on)
  (:Pressed
    (if (Variables|Default|GetbmCanPlayerKick)
      (for _index (range 1 3)
        _))))

(event Input|ActionEvents|InputActionplaceBomb
  (params (Key :type Key%20Structure :default "AnyKey"))
  (bind _bmbombpresent (Variables|Default|GetbmBombPresent))
  ;[1 0.776 0] Bomb Placing
  (:Pressed
    (if (> (Variables|Default|GetbmBombPresent) 0)
      (bind (_bmcanplacebomb _bmbombtransform) (CallFunction|BmGetBombTransform))
      (if _bmcanplacebomb
        (Networking|SwitchHasAuthority
          (:Authority
            (Default|BmPlaceBomb (Variables|Default|GetbmGameStateRef) _bmbombtransform self))
          (:Remote
            (bind _asbomberman_player_controller (Utilities|Casting|CastToBombermanPlayerController (Pawn|GetController)))
            (Default|BmReqPlaceBomb _asbomberman_player_controller _bmbombtransform self)))
        (Development|PrintString (Utilities|String|Append "bomb placed:" (Utilities|String|ToString(Integer) _bmbombpresent)) true true "(R=0.000000,G=0.660000,B=1.000000,A=1.000000)" 5.0)
        (Math|Integer|DecrementInt _bmbombpresent)
        (else
          (Development|PrintString "cant place bomb"))))))

(event Input|AxisEvents|InputAxismoveForward
  (params (AxisValue :type Float%20%28single-precision%29))
  ;[1 1 1] movement setup
  (Pawn|Input|AddMovementInput "1.000000, 0, 0" AxisValue false))

(event Input|AxisEvents|InputAxismoveRight
  (params (AxisValue :type Float%20%28single-precision%29))
  ;[1 1 1] movement setup
  (Pawn|Input|AddMovementInput "0,1.000000, 0" AxisValue false))

(event Input|AxisEvents|InputAxismoveBackward
  (params (AxisValue :type Float%20%28single-precision%29))
  ;[1 1 1] movement setup
  (Pawn|Input|AddMovementInput "-1.000000, 0, 0" AxisValue false))

(event Input|AxisEvents|InputAxismoveLeft
  (params (AxisValue :type Float%20%28single-precision%29))
  ;[1 1 1] movement setup
  (Pawn|Input|AddMovementInput "0,-1.000000, 0" AxisValue false))

(fn ConstructionScript)

(fn BmGetBombTransform
  (bind _returnvalue (Transformation|GetActorRotation))
  (bind _returnvalue_2 (Transformation|GetActorRotation))
  (bind _self self)
  (bind _bmgamestateref (Variables|Default|GetbmGameStateRef))
  (bind _bmgamestateref_2 (Variables|Default|GetbmGameStateRef))
  (bind _yaw (Math|Rotator|BreakRotator _returnvalue))
  (bind _yaw_2 (Math|Rotator|BreakRotator _returnvalue_2))
  (bind (_bmcordx _bmcordy) (Default|BmGetCords _bmgamestateref_2 _self))
  ;[1 1 1] bomb placing snap to grid
  (LocalVariables|SetbmGridX _bmcordx)
  (LocalVariables|SetbmGridY _bmcordy)
  (if (Math|Float|InRange(Float) _yaw -2e+01 2e+01)
    (Math|Integer|IncrementInt (LocalVariables|GetbmGridX)
      (:%20%20
        _)))
  (if (Math|Float|InRange(Float) _yaw 7e+01 1.1e+02)
    (Math|Integer|IncrementInt (LocalVariables|GetbmGridY)
      (:%20%20
        _)))
  (if (Math|Float|InRange(Float) _yaw -1.1e+02 -7e+01)
    (Math|Integer|DecrementInt (LocalVariables|GetbmGridY)
      (:%20%20
        _)))
  (if (or (Math|Float|InRange(Float) _yaw 1.6e+02 1.8e+02) (Math|Float|InRange(Float) _yaw -1.8e+02 -1.6e+02))
    (Math|Integer|DecrementInt (LocalVariables|GetbmGridX)
      (:%20%20
        _)))
  (return (not (Math|Boolean|ORBoolean (Math|Float|InRange(Float) _yaw_2 3e+01 6e+01) (Math|Float|InRange(Float) _yaw_2 1.2e+02 1.5e+02) (Math|Float|InRange(Float) _yaw_2 -6e+01 -3e+01) (Math|Float|InRange(Float) _yaw_2 -1.5e+02 -1.2e+02) (or (Utilities|Array|ContainsItem (Variables|/Game/GameContent/BluePrints/bmGameState.bmGameState_C|GetbmCrateRefArray _bmgamestateref) (Default|BmConverttoCords _bmgamestateref (LocalVariables|GetbmGridX) (LocalVariables|GetbmGridY))) (Utilities|Array|ContainsItem (Variables|/Game/GameContent/BluePrints/bmGameState.bmGameState_C|GetbmFixedBoxRefArray _bmgamestateref) (Default|BmConverttoCords _bmgamestateref (LocalVariables|GetbmGridX) (LocalVariables|GetbmGridY)))))) (Math|Transform|MakeTransform (Math|Vector|MakeVector (Math|Conversions|ToFloat(Integer) (+ (* (LocalVariables|GetbmGridX) 100) 50)) (Math|Conversions|ToFloat(Integer) (+ (* (LocalVariables|GetbmGridY) 100) 50)) 1e+02) "0, 0, 0" (* "1.000000,1.000000,1.000000" 0.7))))