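; Bomb-count pickup trigger that calls IncreaseBombs on the bomberman that overlaps it.
; On any overlap with its CollisionComponent it destroys itself before casting the other actor, so non-bomberman actors also consume it.
; Debug prints report the overlapping actor and the cast result.
; BeginPlay caches the bmGameState, which the overlap logic does not use.
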(event OnComponentBeginOverlap(CollisionComponent)
  (params (OverlappedComponent :type Primitive%20Component%20Object%20Reference) (OtherActor :type Actor%20Object%20Reference) (OtherComp :type Primitive%20Component%20Object%20Reference) (OtherBodyIndex :type Integer) (bFromSweep :type Boolean) (SweepResult :type Hit%20Result%20Structure%20%28by%20ref%29))
  (Actor|DestroyActor)
  (Development|PrintString (Utilities|GetDisplayName OtherActor))
  (bind _asbomberman (Utilities|Casting|CastTobomberman OtherActor)
    (:then
      (Development|PrintString "casted" true true "(R=0.000000,G=0.660000,B=1.000000,A=1.000000)" 1e+01)
      (Default|IncreaseBombs _asbomberman))
    (:CastFailed
      (Development|PrintString "cast failed" true true "(R=1.000000,G=0.000000,B=0.009947,A=1.000000)" 1e+01))))

(event EventBeginPlay
  (bind _asbm_game_state (Utilities|Casting|CastTobmGameState (Game|GetGameState)))
  (Variables|Default|SetbmGameStateRef _asbm_game_state))

(event Collision|EventActorBeginOverlap
  (params (OtherActor :type Actor%20Object%20Reference)))

(event EventTick
  (params (DeltaSeconds :type Float%20%28single-precision%29)))

(fn ConstructionScript)