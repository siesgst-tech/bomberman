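; Bomb actor for a Bomberman-style grid game that detonates three seconds after spawning, returns a bomb to its owning Bomberman and destroys itself.
; BmBombExplosion chains the CheckGrid macro in four directions up to the bomb radius, stopping at map edges or fixed boxes.
; Each reached cell, keyed as X*100+Y in game state, gets an explosion emitter, damages players and destroys crates.
; Detonation also spawns a destructible mesh and short-lived explosion effect.
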(event EventBeginPlay
  (bind _returnvalue (Transformation|GetActorTransform))
  (bind _asbm_game_state (Utilities|Casting|CastTobmGameState (Game|GetGameState)))
  (Variables|Default|SetbmGameStateRef _asbm_game_state)
  (bind _outactors (Actor|GetAllActorsOfClass "/Game/GameContent/BluePrints/bomberman.bomberman_C"))
  (Variables|Default|SetbmPlayerArray _outactors)
  (bind _asbomberman (Utilities|Casting|CastTobomberman (Components|GetOwner)))
  (bind _output_get (Variables|Default|SetbmBombermanRef _asbomberman))
  (bind _asbm_game_instance (Utilities|Casting|CastTobmGameInstance (Game|GetGameInstance)))
  (Variables|Default|SetbmGameInstRef _asbm_game_instance)
  (Utilities|FlowControl|Delay 3.0)
  (Default|IncreaseBombs _output_get)
  (Development|PrintString "bomb increased")
  (CallFunction|BmBombExplosion _returnvalue)
  (Game|SpawnActorfromClass "/Game/GameContent/BluePrints/bmDestructibleBombMeshBP.bmDestructibleBombMeshBP_C" _returnvalue "Undefined" 0 0)
  (bind _returnvalue_2 (Game|SpawnActorfromClass "/Game/StarterContent/Blueprints/Blueprint_Effect_Explosion.Blueprint_Effect_Explosion_C" _returnvalue "Undefined" 0 0))
  (Actor|DestroyActor)
  (Utilities|FlowControl|Delay 0.4)
  (Actor|DestroyActor _returnvalue_2))

(fn ConstructionScript)

(fn BmBombExplosion
  (params (bmBombTransform :type Transform))
  (bind _self self)
  (bind _bmgamestateref (Variables|Default|GetbmGameStateRef))
  (bind (_bmcordx _bmcordy) (Default|BmGetCords _bmgamestateref _self))
  (LocalVariables|SetbmLocalX _bmcordx)
  (LocalVariables|SetbmLocalY _bmcordy)
  (Utilities|CheckGrid (LocalVariables|GetbmLocalX) (LocalVariables|GetbmLocalY) false false
    (:output
      (Utilities|CheckGrid (LocalVariables|GetbmLocalX) (LocalVariables|GetbmLocalY) true false
        (:output
          (Utilities|CheckGrid (LocalVariables|GetbmLocalY) (LocalVariables|GetbmLocalX) false true
            (:output
              (Utilities|CheckGrid (LocalVariables|GetbmLocalY) (LocalVariables|GetbmLocalX) true true))))))))

(fn Incrementordecrement
  (params (Decrement :type Boolean) (value :type Integer) (delta :type Integer))
  (if Decrement
    (return (- value delta))
    (else
      (return (+ value delta)))))

(fn GetXYcoords
  (params (Local1 :type Integer) (Local2 :type Integer) (is%20Y :type Boolean))
  (if is%20Y
    (return (+ Local1 (* Local2 100)))
    (else
      (return (+ Local2 (* Local1 100))))))