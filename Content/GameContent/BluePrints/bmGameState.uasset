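; Game state for a Bomberman-style game that tracks the grid layout and handles bomb placement, explosion effects, crate destruction and power-up removal.
; BeginPlay indexes fixed boxes, crates and power-ups by packing their 100-unit cell coordinates into one integer (X*100+Y).
; Parallel key and actor arrays let events find actors by cell; destroyed crates become destructible meshes and leave both arrays.
; The player-kill event is an empty stub.
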(event Custom|bmPlaceBomb
  (params (bmBombTrans :type Transform) (bomberman :type Bomberman%20Object%20Reference))
  (Game|SpawnActorfromClass "/Game/GameContent/BluePrints/bmBombMeshBP.bmBombMeshBP_C" bmBombTrans "Undefined" bomberman 0))

(event Custom|bmCrateDestruction
  (params (bmCrateCord :type Integer))
  (bind _bmcratemesharray (Variables|Default|GetbmCrateMeshArray))
  (bind _bmcraterefarray (Variables|Default|GetbmCrateRefArray))
  (bind _returnvalue (Utilities|Array|FindItem _bmcraterefarray bmCrateCord))
  (bind _output (Utilities|Array|Get(acopy) _bmcratemesharray _returnvalue))
  (bind _returnvalue_2 (Transformation|GetActorTransform _output))
  (Game|SpawnActorfromClass "/Game/GameContent/BluePrints/bmDestructibleCrateMeshBP.bmDestructibleCrateMeshBP_C" _returnvalue_2 "Undefined" 0 0)
  (Effects|SpawnEmitteratLocation "/Game/StarterContent/Particles/P_Explosion.P_Explosion" (.Location (Math|Transform|BreakTransform _returnvalue_2)))
  (Actor|DestroyActor _output)
  (Utilities|Array|RemoveIndex _bmcratemesharray _returnvalue)
  (Utilities|Array|RemoveIndex (Variables|Default|GetbmCrateRefArray) _returnvalue))

(event Custom|bmDestroyPowerUp
  (params (bmTriggerRef :type Actor%20Object%20Reference))
  (bind (_bmcordx _bmcordy) (CallFunction|BmGetCords bmTriggerRef))
  (bind _bmpoweruprefarray (Variables|Default|GetbmPowerUpRefArray))
  (bind _bmcord (CallFunction|BmConverttoCords _bmcordx _bmcordy))
  (bind _returnvalue (Utilities|Array|FindItem _bmpoweruprefarray _bmcord))
  (if (!= _returnvalue -1)
    (Actor|DestroyActor (Utilities|Array|Get(acopy) (Variables|Default|GetbmPowerUpActorArray) _returnvalue))))

(event Custom|bmPlayerKill)

(event Custom|bmSpawnExplosionEmitter
  (params (Location :type Vector))
  (Effects|SpawnEmitteratLocation "/Game/StarterContent/Particles/P_Explosion.P_Explosion" Location))

(event EventBeginPlay
  (bind _asbomberman (Utilities|Casting|CastTobomberman (Game|GetPlayerCharacter 0)))
  (Variables|Default|SetBombermanRef _asbomberman)
  (bind _outactors (Actor|GetAllActorsOfClass "/Game/GameContent/BluePrints/bmFixedBoxMeshBP.bmFixedBoxMeshBP_C"))
  (for _array_element _outactors
    (Utilities|Array|Add (Variables|Default|GetbmFixedBoxRefArray) (+ (* (.bmCordX (CallFunction|BmGetCords _array_element)) 100) (.bmCordY (CallFunction|BmGetCords _array_element)))))
  (bind _outactors_2 (Actor|GetAllActorsOfClass "/Game/GameContent/BluePrints/bmCrateMeshBP.bmCrateMeshBP_C"))
  (bind _output_get (Variables|Default|SetbmCrateMeshArray _outactors_2))
  (for (_array_element_2 _array_index) _output_get
    (Utilities|Array|Insert (Variables|Default|GetbmCrateRefArray) (+ (* (.bmCordX (CallFunction|BmGetCords _array_element_2)) 100) (.bmCordY (CallFunction|BmGetCords _array_element_2))) _array_index))
  (bind _outactors_3 (Actor|GetAllActorsOfClass "/Game/GameContent/BluePrints/bmPowerupBP.bmPowerupBP_C"))
  (bind _output_get_2 (Variables|Default|SetbmPowerUpActorArray _outactors_3))
  (for (_array_element_3 _array_index_2) _output_get_2
    (Utilities|Array|Insert (Variables|Default|GetbmPowerUpRefArray) (CallFunction|BmConverttoCords (.bmCordX (CallFunction|BmGetCords _array_element_3)) (.bmCordY (CallFunction|BmGetCords _array_element_3))) _array_index_2)))

(fn ConstructionScript)

(fn BmGetCords
  (params (bmActor :type Actor%20Object%20Reference))
  (bind _returnvalue (Transformation|GetActorTransform bmActor))
  (bind _location (Math|Transform|BreakTransform _returnvalue))
  (bind (_x _y) (Math|Vector|BreakVector _location))
  (return (.ReturnValue (Math|Float|Division(WholeandRemainder) _x 1e+02)) (.ReturnValue (Math|Float|Division(WholeandRemainder) _y 1e+02))))

(fn BmGetTransform
  (params (bmCords :type Integer))
  (return (Math|Transform|MakeTransform (Math|Vector|MakeVector (Math|Conversions|ToFloat(Integer) (+ (* (/ bmCords 100) 100) 50)) (Math|Conversions|ToFloat(Integer) (+ (* (Math|Integer|%(Integer) bmCords 100) 100) 50)) 0.0))))

(fn BmConverttoCords
  (params (bmCordX :type Integer) (bmCordY :type Integer))
  (return (+ (* bmCordX 100) bmCordY)))