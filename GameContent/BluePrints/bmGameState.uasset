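; Bomberman game state Blueprint that tracks the grid of fixed boxes and crates and handles bombs and player deaths.
; On BeginPlay it packs each box and crate's 100-unit cell position into an integer (X*100+Y), indexing crates alongside their mesh actors.
; Explosion events swap the crate at a given coordinate for a destructible mesh with an emitter and unregister it.
; Other events spawn bombs and decrement player life, printing on death.
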(event Custom|bmPlaceBomb
  (params (bmBombTrans :type Transform))
  (Game|SpawnActorfromClass "/Game/GameContent/BluePrints/bmBombMeshBP.bmBombMeshBP_C" bmBombTrans "Undefined" 0 0))

(event Custom|bmExplodeBomb
  (params (bmCrateCord :type Integer))
  (bind _bmcratemesharray (Variables|Default|GetbmCrateMeshArray))
  (bind _bmcraterefarray (Variables|Default|GetbmCrateRefArray))
  (bind _returnvalue (Utilities|Array|FindItem _bmcraterefarray bmCrateCord))
  (bind _output (Utilities|Array|Get(acopy) _bmcratemesharray _returnvalue))
  (bind _returnvalue_2 (Transformation|GetActorTransform _output))
  (Game|SpawnActorfromClass "/Game/GameContent/BluePrints/bmDestructibleCrateMeshBP.bmDestructibleCrateMeshBP_C" _returnvalue_2 "Undefined" 0 0)
  (Effects|SpawnEmitteratLocation "/Game/StarterContent/Particles/P_Explosion.P_Explosion" (.Location (Math|Transform|BreakTransform _returnvalue_2)))
  (Actor|DestroyActor _output)
  (Utilities|Array|RemoveIndex _bmcratemesharray _returnvalue)
  (Utilities|Array|RemoveIndex (Variables|Default|GetbmCrateRefArray) _returnvalue))

(event Custom|bmPlayerKill
  (bind _result (Math|Integer|DecrementInt (Variables|/Game/GameContent/BluePrints/bomberman.bomberman_C|GetbmPlayerLife (Variables|Default|GetbmBombermanRef)))
    (:%20%20
      (if (> _result 0)
        _
        (else
          ;[1 1 1] game over condition
          (Development|PrintString "player dead")))
      (Development|PrintString (Utilities|String|Append "player life  " (Utilities|String|ToString(Integer) _result))))))

(event EventBeginPlay
  (bind _asbomberman (Utilities|Casting|CastTobomberman (Game|GetPlayerCharacter 0)))
  (Variables|Default|SetbmBombermanRef _asbomberman)
  (bind _outactors (Actor|GetAllActorsOfClass "/Game/GameContent/BluePrints/bmFixedBoxMeshBP.bmFixedBoxMeshBP_C"))
  (for _array_element _outactors
    (Utilities|Array|Add (Variables|Default|GetbmFixedBoxRefArray) (+ (* (.bmCordX (CallFunction|BmGetCords _array_element)) 100) (.bmCordY (CallFunction|BmGetCords _array_element)))))
  (bind _outactors_2 (Actor|GetAllActorsOfClass "/Game/GameContent/BluePrints/bmCrateMeshBP.bmCrateMeshBP_C"))
  (bind _output_get (Variables|Default|SetbmCrateMeshArray _outactors_2))
  (for (_array_element_2 _array_index) _output_get
    (Utilities|Array|Insert (Variables|Default|GetbmCrateRefArray) (+ (* (.bmCordX (CallFunction|BmGetCords _array_element_2)) 100) (.bmCordY (CallFunction|BmGetCords _array_element_2))) _array_index)))

(fn ConstructionScript)

(fn BmGetCords
  (params (bmActor :type Actor%20Object%20Reference))
  (bind _returnvalue (Transformation|GetActorTransform bmActor))
  (bind _location (Math|Transform|BreakTransform _returnvalue))
  (bind (_x _y) (Math|Vector|BreakVector _location))
  (return (.ReturnValue (Math|Float|Division(WholeandRemainder) _x 1e+02)) (.ReturnValue (Math|Float|Division(WholeandRemainder) _y 1e+02))))

(fn BmGetTransform
  (params (bmCords :type Integer))
  (return (Math|Transform|MakeTransform (Math|Vector|MakeVector (Math|Conversions|ToFloat(Integer) (* (/ bmCords 100) 100)) (Math|Conversions|ToFloat(Integer) (* (Math|Integer|%(Integer) bmCords 100) 100)) 0.0))))

(fn BmConverttoCords
  (params (bmCordX :type Integer) (bmCordY :type Integer))
  (return (+ (* bmCordX 100) bmCordY)))