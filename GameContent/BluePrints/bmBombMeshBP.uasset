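; Bomb actor for a grid-based, Bomberman-style game that explodes in a cross pattern shortly after spawning.
; BeginPlay waits briefly, spawns a destructible bomb mesh, increments the game instance's bomb count, runs the explosion and destroys itself.
; The explosion walks the game state's flattened grid in four directions up to the bomb radius, stopping at blocking cells or map bounds and passing destructible cells to the game state.
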(event EventBeginPlay
  (bind _asbm_game_state (Utilities|Casting|CastTobmGameState (Game|GetGameState)))
  (Variables|Default|SetbmGameStateRef _asbm_game_state)
  (Utilities|FlowControl|Delay 1.0)
  (Game|SpawnActorfromClass "/Game/GameContent/BluePrints/bmDestructibleBombMeshBP.bmDestructibleBombMeshBP_C" (Transformation|GetWorldTransform (Variables|Default|GetStaticMesh)) "Undefined" 0 0)
  (bind _asbm_game_instance (Utilities|Casting|CastTobmGameInstance (Game|GetGameInstance)))
  (bind _output_get (Variables|Default|SetbmGameInstRef _asbm_game_instance))
  (Variables|/Game/GameContent/BluePrints/bmGameInstance.bmGameInstance_C|SetbmBombPresent _output_get (+ (Variables|/Game/GameContent/BluePrints/bmGameInstance.bmGameInstance_C|GetbmBombPresent _asbm_game_instance) 1))
  (CallFunction|BmBombExplosion (Transformation|GetActorTransform))
  (Actor|DestroyActor))

(fn ConstructionScript)

(fn IsinRangeCrate
  (params (bmCrateMesh :type Actor%20Object%20Reference) (bmBombMesh :type Actor%20Object%20Reference) (bmRangeMultiplier :type Integer))
  (bind _returnvalue (Transformation|GetActorTransform bmCrateMesh))
  (bind _returnvalue_2 (* bmRangeMultiplier 2e+02))
  (bind _staticmesh (Variables|Default|GetStaticMesh))
  (bind _returnvalue_3 (Components|GetOwner _staticmesh))
  (bind _location (Math|Transform|BreakTransform _returnvalue))
  (bind (_x _y) (Math|Vector|BreakVector _location))
  (bind _returnvalue_4 (Transformation|GetActorTransform _returnvalue_3))
  (bind _location_2 (Math|Transform|BreakTransform _returnvalue_4))
  (bind (_x_2 _y_2) (Math|Vector|BreakVector _location_2))
  (return (and (<= (Math|Float|Absolute(Float) (- _x _x_2)) _returnvalue_2) (<= (Math|Float|Absolute(Float) (- _y _y_2)) _returnvalue_2))))

(fn BmBombExplosion
  (params (bmBoMbTransform :type Transform))
  (bind _bmgameinstref (Variables|Default|GetbmGameInstRef))
  (bind _bmgameinstref_2 (Variables|Default|GetbmGameInstRef))
  (bind _bmgameinstref_3 (Variables|Default|GetbmGameInstRef))
  (bind _bmgameinstref_4 (Variables|Default|GetbmGameInstRef))
  (bind _bmmapsize (Variables|/Game/GameContent/BluePrints/bmGameInstance.bmGameInstance_C|GetbmMapSIze _bmgameinstref))
  (bind _bmmapsize_2 (Variables|/Game/GameContent/BluePrints/bmGameInstance.bmGameInstance_C|GetbmMapSIze _bmgameinstref_3))
  (bind _bmmapsize_3 (Variables|/Game/GameContent/BluePrints/bmGameInstance.bmGameInstance_C|GetbmMapSIze _bmgameinstref_2))
  (bind _bmmapsize_4 (Variables|/Game/GameContent/BluePrints/bmGameInstance.bmGameInstance_C|GetbmMapSIze _bmgameinstref_4))
  (bind (_bmgridx _bmgridy) (Default|BmGetPlayerGrid (Variables|Default|GetbmGameStateRef) bmBoMbTransform))
  (LocalVariables|SetbmLocalX _bmgridx)
  (LocalVariables|SetbmLocalY _bmgridy)
  ;[1 1 1] checking positive X
  (LocalVariables|SetbmCheckGrid (+ (LocalVariables|GetbmLocalX) (* (LocalVariables|GetbmLocalY) _bmmapsize_2)))
  (Utilities|FlowControl|ForLoopwithBreak 1 (Variables|Default|GetbmBombRadius) :!label _label
    (:LoopBody
      (if (<= (+ (LocalVariables|GetbmCheckGrid) _bmmapsize_2) (- (* _bmmapsize_3 _bmmapsize_3) 1))
        (bind _output_get (LocalVariables|SetbmCheckGrid (+ (LocalVariables|GetbmCheckGrid) _bmmapsize_2)))
        (switch int (Utilities|Array|Get(acopy) (Variables|/Game/GameContent/BluePrints/bmGameState.bmGameState_C|GetbmGridRefArray (Variables|Default|GetbmGameStateRef)) _output_get)
          (:1
            (goto _label Break))
          (:2
            (Default|BmBombExplosion (Variables|Default|GetbmGameStateRef) (LocalVariables|GetbmCheckGrid))))
        (else
          (goto _label Break))))
    (:Completed
      ;[1 1 1] checking negative X
      (LocalVariables|SetbmCheckGrid (+ (LocalVariables|GetbmLocalX) (* (LocalVariables|GetbmLocalY) _bmmapsize)))
      (Utilities|FlowControl|ForLoopwithBreak 1 (Variables|Default|GetbmBombRadius) :!label _label_2
        (:LoopBody
          (if (>= (- (LocalVariables|GetbmCheckGrid) _bmmapsize) 0)
            (bind _output_get_2 (LocalVariables|SetbmCheckGrid (- (LocalVariables|GetbmCheckGrid) _bmmapsize)))
            (switch int (Utilities|Array|Get(acopy) (Variables|/Game/GameContent/BluePrints/bmGameState.bmGameState_C|GetbmGridRefArray (Variables|Default|GetbmGameStateRef)) _output_get_2)
              (:1
                (goto _label_2 Break))
              (:2
                (Default|BmBombExplosion (Variables|Default|GetbmGameStateRef) (LocalVariables|GetbmCheckGrid))))
            (else
              (goto _label_2 Break))))
        (:Completed
          ;[1 1 1] checking positive Y
          (bind _output_get_3 (LocalVariables|SetbmCheckGrid (+ (LocalVariables|GetbmLocalX) (* (LocalVariables|GetbmLocalY) (Variables|/Game/GameContent/BluePrints/bmGameInstance.bmGameInstance_C|GetbmMapSIze (Variables|Default|GetbmGameInstRef))))))
          (Utilities|FlowControl|ForLoopwithBreak 1 (Variables|Default|GetbmBombRadius) :!label _label_3
            (:LoopBody
              (if (<= (+ (LocalVariables|GetbmCheckGrid) 1) (+ _bmmapsize_4 (- _output_get_3 (Math|Integer|%(Integer) _output_get_3 _bmmapsize_4))))
                (bind _output_get_4 (LocalVariables|SetbmCheckGrid (+ (LocalVariables|GetbmCheckGrid) 1)))
                (switch int (Utilities|Array|Get(acopy) (Variables|/Game/GameContent/BluePrints/bmGameState.bmGameState_C|GetbmGridRefArray (Variables|Default|GetbmGameStateRef)) _output_get_4)
                  (:1
                    (goto _label_3 Break))
                  (:2
                    (Default|BmBombExplosion (Variables|Default|GetbmGameStateRef) (LocalVariables|GetbmCheckGrid))))
                (else
                  (goto _label_3 Break))))
            (:Completed
              ;[1 1 1] checking negative Y
              (bind _output_get_5 (LocalVariables|SetbmCheckGrid (+ (LocalVariables|GetbmLocalX) (* (LocalVariables|GetbmLocalY) (Variables|/Game/GameContent/BluePrints/bmGameInstance.bmGameInstance_C|GetbmMapSIze (Variables|Default|GetbmGameInstRef))))))
              (Utilities|FlowControl|ForLoopwithBreak 1 (Variables|Default|GetbmBombRadius) :!label _label_4
                (:LoopBody
                  (if (>= (- (LocalVariables|GetbmCheckGrid) 1) (- _output_get_5 (Math|Integer|%(Integer) _output_get_5 (Variables|/Game/GameContent/BluePrints/bmGameInstance.bmGameInstance_C|GetbmMapSIze (Variables|Default|GetbmGameInstRef)))))
                    (bind _output_get_6 (LocalVariables|SetbmCheckGrid (- (LocalVariables|GetbmCheckGrid) 1)))
                    (switch int (Utilities|Array|Get(acopy) (Variables|/Game/GameContent/BluePrints/bmGameState.bmGameState_C|GetbmGridRefArray (Variables|Default|GetbmGameStateRef)) _output_get_6)
                      (:1
                        (goto _label_4 Break))
                      (:2
                        (Default|BmBombExplosion (Variables|Default|GetbmGameStateRef) (LocalVariables|GetbmCheckGrid))))
                    (else
                      (goto _label_4 Break))))))))))))