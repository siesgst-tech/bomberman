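; Player Blueprint for a Bomberman-style game, handling movement and bomb placement.
; Axis inputs move it relative to control yaw; placeBomb spawns a BmBombMeshBP while BombsPresent is above zero, then decrements that count.
; BmGetBombTransform is unfinished: it always allows placement at a fixed X/Y origin, scaled from BmBombScale.
; Facing-based grid targeting, the BmBombScale update and mouse-look nodes are disconnected.
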(event Input|ActionEvents|InputActionplaceBomb
  (params (Key :type Key%20Structure :default "AnyKey"))
  ;[1 1 1] Working Code works for multiple bombs
  (:Pressed
    (if (> (Variables|Default|GetBombsPresent) 0)
      (bind (_bmcanplacebomb _bmplayertransform) (CallFunction|BmGetBombTransform))
      (if _bmcanplacebomb
        (Game|SpawnActorfromClass "/Game/GameContent/BluePrints/bmBombMeshBP.bmBombMeshBP_C" _bmplayertransform "AdjustIfPossibleButDontSpawnIfColliding" 0 0)
        (Variables|Default|SetBombsPresent (- (Variables|Default|GetBombsPresent) 1))
        (Development|PrintString "bomb placed")))))

(event Input|AxisEvents|InputAxismoveForward
  (params (AxisValue :type Float%20%28single-precision%29))
  ;[1 1 1] all the easy stuff
  ;;[1 1 1] movement setup
  (Pawn|Input|AddMovementInput (Math|Vector|GetForwardVector (Math|Rotator|MakeRotator 0.0 0.0 (.Yaw (Math|Rotator|BreakRotator (Pawn|GetControlRotation :!class /Script/Engine.Pawn))))) AxisValue false))

(event Input|AxisEvents|InputAxismoveRight
  (params (AxisValue :type Float%20%28single-precision%29))
  ;[1 1 1] all the easy stuff
  ;;[1 1 1] movement setup
  (Pawn|Input|AddMovementInput (Math|Vector|GetRightVector (Math|Rotator|MakeRotator 0.0 0.0 (.Yaw (Math|Rotator|BreakRotator (Pawn|GetControlRotation :!class /Script/Engine.Pawn))))) AxisValue false))

(fn ConstructionScript)

(fn BmGetBombTransform
  (return true (Math|Transform|MakeTransform (Math|Vector|MakeVector (- 0.0 0.0) (- 0.0 0.0) 7e+01) "0, 0, 0" (* (LocalVariables|GetbmBombScale) 0.7))))